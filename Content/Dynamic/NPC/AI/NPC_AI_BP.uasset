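; NPC AI controller Blueprint that runs guard behavior for an NPC and reacts to what it perceives.
; On BeginPlay it sets up the PatrolData blackboard and runs the GuardBehaviour tree.
; AI Perception updates write any sensed actor lacking the "Enemy" tag into the blackboard's enemy key.
; Losing sight or sense of any such actor clears that key, without checking whether it was the stored target.
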(event OnTargetPerceptionUpdated(AIPerception)
  (params (Actor :type Actor%20Object%20Reference) (Stimulus :type AI%20Stimulus%20Structure))
  (bind _enemy_key (Variables|Default|GetEnemy%20Key))
  (bind _blackboard_comp (Variables|Default|GetBlackboard%20Comp))
  (if (not (Actor|ActorHasTag Actor "Enemy"))
    (if (.bSuccessfullySensed (Utilities|Struct|BreakAIStimulus Stimulus))
      (AI|Components|Blackboard|SetValueasObject _blackboard_comp _enemy_key Actor)
      (else
        (AI|Components|Blackboard|ClearValue _blackboard_comp _enemy_key)))))

(event EventBeginPlay
  (bind _blackboardcomponent (Class|AIController|UseBlackboard "/Game/Dynamic/NPC/AI/PatrolData.PatrolData"))
  (AI|RunBehaviorTree "/Game/Dynamic/NPC/AI/GuardBehaviour.GuardBehaviour")
  (Variables|Default|SetBlackboard%20Comp _blackboardcomponent))

(fn ConstructionScript)